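; Base player controller that creates the primary UI widget and routes input for movement, camera, jump, melee and abilities to the controlled pawn.
; Movement follows camera rotation, and Cancel calls TargetCancel on the character's Ability System Component.
; Five slot inputs look up an ability class in the UI widget and activate it by class through GAS.
; Slot activation also flags targeting abilities, calls TargetCancel and ends the melee combo.
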(event `self.ReceiveBeginPlay`
  (bind _returnvalue (`|CreateWidget` "/Game/UI/WBP_PrimaryUI.WBP_PrimaryUI_C"))
  (bind _output_get (set `self.PrimaryUIWidget` _returnvalue))
  (`UserWidget.AddToViewport` _output_get 0))

(event `InputAxis|MoveForward`
  (params (AxisValue :type "Float (single-precision)"))
  ;[1 1 1] Basic Controll Setup
  (`Pawn.AddMovementInput` (`self.K2_GetPawn`) (`KismetMathLibrary.GetForwardVector` (`PlayerCameraManager.GetCameraRotation` (`self.PlayerCameraManager`))) AxisValue false))

(event `InputAxis|MoveRight`
  (params (AxisValue :type "Float (single-precision)"))
  ;[1 1 1] Basic Controll Setup
  (`Pawn.AddMovementInput` (`self.K2_GetPawn`) (`KismetMathLibrary.GetRightVector` (`PlayerCameraManager.GetCameraRotation` (`self.PlayerCameraManager`))) AxisValue false))

(event `InputAction|Jump`
  (params (Key :type "Key Structure"))
  ;[1 1 1] Basic Controll Setup
  (:`Pressed`
    (bind _ascharacter (cast `Character` (`self.K2_GetPawn`)))
    (`Character.Jump` _ascharacter)))

(event `InputAxis|LookUp`
  (params (AxisValue :type "Float (single-precision)"))
  ;[1 1 1] Basic Controll Setup
  (`self.AddPitchInput` AxisValue))

(event `InputAxis|LookRight`
  (params (AxisValue :type "Float (single-precision)"))
  ;[1 1 1] Basic Controll Setup
  (`self.AddYawInput` AxisValue))

(event `self.AddAbilityToUI`
  (params (AbilityInfo :type "GamePlayAbilityInfo Structure"))
  (`/Game/UI/WBP_PrimaryUI.AddAbilitiesToSlots` (`self.PrimaryUIWidget`) AbilityInfo))

(event `InputAction|PrimaryAction`
  (params (Key :type "Key Structure"))
  ;[1 1 1] Ability Control Setup
  (:`Pressed`
    (bind _asbp_base_character (cast `/Game/Blueprints/Characters/BP_BaseCharacter` (`self.K2_GetPawn`)))
    (`/Game/Blueprints/Characters/BP_BaseCharacter.MeleeAttack` _asbp_base_character)))

(event `InputAction|Cancel`
  (params (Key :type "Key Structure"))
  ;[1 1 1] Ability Control Setup
  (:`Pressed`
    (bind _asbp_base_character (cast `/Game/Blueprints/Characters/BP_BaseCharacter` (`self.K2_GetPawn`)))
    (`AbilitySystemComponent.TargetCancel` (`AbilitySystemBlueprintLibrary.GetAbilitySystemComponent` _asbp_base_character))))

(event `InputAction|AbilityOneSlot`
  (params (Key :type "Key Structure"))
  ;[1 1 1] Ability Control Setup
  (:`Pressed`
    (`self.TryActivateAbilitySlotByClass` 0)))

(event `InputAction|AbilityTwoSlot`
  (params (Key :type "Key Structure"))
  ;[1 1 1] Ability Control Setup
  (:`Pressed`
    (`self.TryActivateAbilitySlotByClass` 1)))

(event `InputAction|AbilityThreeSlot`
  (params (Key :type "Key Structure"))
  ;[1 1 1] Ability Control Setup
  (:`Pressed`
    (`self.TryActivateAbilitySlotByClass` 2)))

(event `InputAction|AbilityFourSlot`
  (params (Key :type "Key Structure"))
  ;[1 1 1] Ability Control Setup
  (:`Pressed`
    (`self.TryActivateAbilitySlotByClass` 3)))

(event `InputAction|AbilityFiveSlot`
  (params (Key :type "Key Structure"))
  ;[1 1 1] Ability Control Setup
  (:`Pressed`
    (`self.TryActivateAbilitySlotByClass` 4)))

(fn `TryActivateAbilitySlotByClass`
  (params (SlotIndex :type Integer))
  (bind (_ability _valid) (`/Game/UI/WBP_PrimaryUI.GetAbilityClassSlot` (`self.PrimaryUIWidget`) SlotIndex))
  (if _valid
    (bind _asbp_base_character (cast `/Game/Blueprints/Characters/BP_BaseCharacter` (`self.K2_GetPawn`)))
    (bind _returnvalue (`AbilitySystemBlueprintLibrary.GetAbilitySystemComponent` _asbp_base_character))
    (`AbilitySystemComponent.TryActivateAbilityByClass` _returnvalue _ability true)
    (castclass `/Game/Blueprints/Characters/Abilities/GA_BaseClassTargeting` _ability
      (:`then`
        (set `/Game/Blueprints/Characters/BP_BaseCharacter.IsTargeting` true _asbp_base_character))
      (:`CastFailed`
        (set `/Game/Blueprints/Characters/BP_BaseCharacter.IsTargeting` false _asbp_base_character)))
    (`AbilitySystemComponent.TargetCancel` _returnvalue)
    (set `self.IsGroundBlastActivated` true)
    (`/Game/Blueprints/Characters/BP_BaseCharacter.EndCombo` _asbp_base_character)))

(fn `UserConstructionScript`)