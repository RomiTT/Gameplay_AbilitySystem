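; Base gameplay ability Blueprint providing shared helpers for character abilities, with no activation logic of its own.
; A lookup casts the owning actor to BP_BaseCharacter and its controller to BP_PlayerControllerBase, feeding the other helpers.
; StartUICooldown starts cooldown on the primary UI slot whose ability class matches GetAbilityInfo.
; CanContinueCastingAbility checks that current Health, Mana or Strength, chosen by cost type, exceeds the negated cost.
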(fn `CanContinueCastingAbility`
  (returns (Can :type Boolean))
  (locals (`Cost ` :type "Float (double-precision)"))
  (bind (_strength_basevalue _strength_currentvalue) (break `GameplayAttributeData` (`ASAttributeSetBase.Strength` (`ASCharacterBase.AttributeSetBaseComp` (`self.GetCharacterBaseAndPlayerController`)))))
  (bind (_health_basevalue _health_currentvalue) (break `GameplayAttributeData` (`ASAttributeSetBase.Health` (`ASCharacterBase.AttributeSetBaseComp` (`self.GetCharacterBaseAndPlayerController`)))))
  (bind (_mana_basevalue _mana_currentvalue) (break `GameplayAttributeData` (`ASAttributeSetBase.Mana` (`ASCharacterBase.AttributeSetBaseComp` (`self.GetCharacterBaseAndPlayerController`)))))
  (bind _returnvalue (`self.GetAbilityInfo`))
  (set `local.Cost ` (* (`.Cost` (break `GamePlayAbilityInfo` _returnvalue)) -1.0))
  (switch `EAbilityCostType` (`.CostType` (break `GamePlayAbilityInfo` _returnvalue))
    (:`Health`
      (return (> _health_currentvalue (`local.Cost `))))
    (:`Mana`
      (return (> _mana_currentvalue (`local.Cost `))))
    (:`Strength`
      (return (> _strength_currentvalue (`local.Cost `))))))

(fn `GetCharacterBaseAndPlayerController`
  (returns (CharacterBase :type "/Game/Blueprints/Characters/BP_BaseCharacter Object Reference") (PlayerController :type "/Game/Blueprints/BP_PlayerControllerBase Object Reference"))
  (bind _asbp_base_character (cast `/Game/Blueprints/Characters/BP_BaseCharacter` (`self.GetOwningActorFromActorInfo`)))
  (`/Engine/EditorBlueprintResources/StandardMacros.IsValid` _asbp_base_character
    (:`Is Valid`
      (bind _asbp_player_controller_base (cast `/Game/Blueprints/BP_PlayerControllerBase` (`Pawn.GetController` _asbp_base_character)))
      (return _asbp_base_character _asbp_player_controller_base))))

(fn `StartUICooldown`
  (bind (_characterbase _playercontroller) (`self.GetCharacterBaseAndPlayerController`))
  (`/Engine/EditorBlueprintResources/StandardMacros.IsValid` _playercontroller
    (:`Is Valid`
      (for _array_element (`/Game/UI/WBP_PrimaryUI.AbilitySlots` (`/Game/Blueprints/BP_PlayerControllerBase.PrimaryUIWidget` _playercontroller))
        (bind _returnvalue (`self.GetAbilityInfo`))
        (bind (_abilityinfo_cooldownduration _abilityinfo_cost _abilityinfo_uimat _abilityinfo_costtype _abilityinfo_abilityclass) (break `GamePlayAbilityInfo` (`/Game/UI/WBP_AbilitySlot.AbilityInfo` _array_element)))
        (if (== _abilityinfo_abilityclass (`.AbilityClass` (break `GamePlayAbilityInfo` _returnvalue)))
          (`/Game/UI/WBP_AbilitySlot.StartCooldown` _array_element)
          (return))))))