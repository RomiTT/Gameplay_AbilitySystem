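; Base character Blueprint that drives Gameplay Ability System combat: melee, dash and health regen, plus death and knockback handling.
; It grants abilities at BeginPlay, activates them by class, and confirms targeting on melee input while targeting.
; Sword and capsule overlaps with hostile characters send gameplay events for damage, with the dash excluding repeat hits.
; Helpers cycle a three-step melee combo, toggle camera-driven rotation, and apply a frictionless impulse push with stun.
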(event `self.ReceiveBeginPlay`
  ;[1 1 1] Aquiring the ability to our Player
  (`self.AquireAbilities` (`self.AbilitiesClass`)))

(event `MeleeAttack`
  ;[1 1 1] Single Attack Using left click
  (if (`self.IsTargeting`)
    (`AbilitySystemComponent.TargetConfirm` (`self.AbilitySystemComp`))
    (else
      (`AbilitySystemComponent.TryActivateAbilityByClass` (`self.AbilitySystemComp`) "/Game/Blueprints/Characters/Abilities/Melee/GA_Melee.GA_Melee_C" true))))

(event `self.SwordCollision.OnComponentBeginOverlap`
  (params (OverlappedComponent :type "PrimitiveComponent Object Reference") (OtherActor :type "Actor Object Reference") (OtherComp :type "PrimitiveComponent Object Reference") (OtherBodyIndex :type Integer) (bFromSweep :type Boolean) (SweepResult :type "HitResult Structure (by ref)"))
  ;[1 1 1] Sending the gameplay event data to the actor that we wanna deal with
  (bind _asbp_base_character (cast `/Game/Blueprints/Characters/BP_BaseCharacter` OtherActor))
  (if (and (`self.IsOtherHostile` _asbp_base_character self) (!= self OtherActor))
    (`AbilitySystemBlueprintLibrary.SendGameplayEventToActor` self (struct :`TagName` "ability.melee.dealDamage") (make `GameplayEventData` (struct) null OtherActor))))

(event `HealthRegen`
  ;[1 1 1] Health Regen Using 1 in keyboard
  (`AbilitySystemComponent.TryActivateAbilityByClass` (`self.AbilitySystemComp`) "/Game/Blueprints/Characters/Abilities/HealthRegen/GA_HealthRegen.GA_HealthRegen_C" true))

(event `self.CapsuleComponent.OnComponentBeginOverlap`
  (params (OverlappedComponent :type "PrimitiveComponent Object Reference") (OtherActor :type "Actor Object Reference") (OtherComp :type "PrimitiveComponent Object Reference") (OtherBodyIndex :type Integer) (bFromSweep :type Boolean) (SweepResult :type "HitResult Structure (by ref)"))
  (bind _asbp_base_character (cast `/Game/Blueprints/Characters/BP_BaseCharacter` OtherActor))
  (if (`self.IsOtherHostile` _asbp_base_character self)
    (if (not (`KismetArrayLibrary.Array_Contains` (`self.OverlappedExeclude`) _asbp_base_character))
      (`KismetArrayLibrary.Array_AddUnique` (`self.OverlappedExeclude`) _asbp_base_character)
      (`AbilitySystemBlueprintLibrary.SendGameplayEventToActor` self (struct :`TagName` "ability.dash.dealDamage") (make `GameplayEventData` (struct) self OtherActor)))))

(event `DashAbility`
  (`AbilitySystemComponent.TryActivateAbilityByClass` (`self.AbilitySystemComp`) "/Game/Blueprints/Characters/Abilities/Dash/GA_Dash.GA_Dash_C" true))

(event `self.BP_StartDyingSequence`
  ;[1 1 1] Start Dying Sequence ( C++ )
  (bind _returnvalue (`self.PlayAnimMontage` "/Game/Blueprints/Characters/Animations/AM_Die_Shinbi.AM_Die_Shinbi"))
  (`self.SetLifeSpan` _returnvalue))

(event `PushAndStun`
  (params (ImpulseDIrection :type "Vector Structure") (ImpulseStrength :type "Float (double-precision)") (StunDuration :type "Float (double-precision)") (TargetController :type "/Game/Blueprints/BP_PlayerControllerBase Object Reference") (AnimMontage :type "AnimMontage Object Reference"))
  (bind _charactermovement (`self.CharacterMovement`))
  (`self.EndCombo`)
  (`self.SetCollisionToPawn` "ECR_Ignore")
  (`self.PlayAnimMontage` AnimMontage)
  (set `self.OriginalGroundFriction` (`CharacterMovementComponent.GroundFriction` (`self.CharacterMovement`)))
  (set `CharacterMovementComponent.GroundFriction` 0.0 _charactermovement)
  (`CharacterMovementComponent.AddImpulse` _charactermovement (* ImpulseDIrection ImpulseStrength) true)
  (`self.Stun` 3.0)
  (`self.SetCollisionToPawn` "ECR_Block"))

(event `EndCombo`
  (set `self.ComboCount` 1))

(fn `DetermineCombo`
  (switch `int` (`self.ComboCount`)
    (:`1`
      (set `self.AnimMontage_CurrentMeleeCombo` "/Game/Blueprints/Characters/Animations/MeleeMontages/AM_Shinbi_Melee_Combo_01.AM_Shinbi_Melee_Combo_01")
      (`/Engine/EditorBlueprintResources/StandardMacros.IncrementInt` (`self.ComboCount`)
        (:`  `
          (set `self.MeleeComboDamageEffectLevel` 1))))
    (:`2`
      (set `self.AnimMontage_CurrentMeleeCombo` "/Game/Blueprints/Characters/Animations/MeleeMontages/AM_Shinbi_Melee_Combo_03.AM_Shinbi_Melee_Combo_03")
      (`/Engine/EditorBlueprintResources/StandardMacros.IncrementInt` (`self.ComboCount`)
        (:`  `
          (set `self.MeleeComboDamageEffectLevel` 2))))
    (:`3`
      (set `self.AnimMontage_CurrentMeleeCombo` "/Game/Blueprints/Characters/Animations/MeleeMontages/AM_Shinbi_Melee_Combo_02.AM_Shinbi_Melee_Combo_02")
      (set `self.ComboCount` 1)
      (set `self.MeleeComboDamageEffectLevel` 3))))

(fn `SetCollisionToPawn`
  (params (`New Collision` :type "ECollisionResponse Enum" :default "ECR_Ignore"))
  (`PrimitiveComponent.SetCollisionResponseToChannel` (`self.CapsuleComponent`) "ECC_Pawn" `New Collision`))

(fn `ShouldCameraControl`
  (params (`Should Control ` :type Boolean))
  (if `Should Control `
    (set `self.bUseControllerRotationYaw` true)
    (set `CharacterMovementComponent.bOrientRotationToMovement` false (`self.CharacterMovement`))
    (else
      (set `self.bUseControllerRotationYaw` false)
      (set `CharacterMovementComponent.bOrientRotationToMovement` true (`self.CharacterMovement`)))))

(fn `UserConstructionScript`)